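; Needle trap actor that repeatedly moves its needles up and down and damages the player on contact.
; A looping event started at BeginPlay plays the NEEDLE timeline to lerp the needle mesh's relative height, then restarts after a short delay.
; On a hit with the player's capsule, it applies damage and forwards the result to ThirdPersonCharacter's ReceiveDamagePlayer.
; The needle moves without sweep.
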(event Custom|NEEDLE_TRAP
  (bind _needle (Timeline|NEEDLE PlayFromStart)
    (:Update
      (Transformation|SetRelativeLocation (Variables|Default|Getneedletrap_Needle) (Math|Vector|Lerp(Vector) "-0.000000,0.000000,-60.000000" "0, 0, 0" _needle) false false))
    (:Finished
      (Utilities|FlowControl|Delay 0.4)
      (CallFunction|NEEDLETRAP))))

(event EventBeginPlay
  (CallFunction|NEEDLETRAP))

(event Collision|EventActorBeginOverlap
  (params (OtherActor :type Actor%20Object%20Reference)))

(event EventTick
  (params (DeltaSeconds :type Float%20%28single-precision%29)))

(event Collision|EventHit
  (params (MyComp :type Primitive%20Component%20Object%20Reference) (Other :type Actor%20Object%20Reference) (OtherComp :type Primitive%20Component%20Object%20Reference) (bSelfMoved :type Boolean) (HitLocation :type Vector :default "0, 0, 0") (HitNormal :type Vector :default "0, 0, 0") (NormalImpulse :type Vector :default "0, 0, 0") (Hit :type Hit%20Result%20Structure%20%28by%20ref%29))
  (if (== OtherComp (Variables|/Script/Engine.Character|GetCapsuleComponent (Game|GetPlayerCharacter 0)))
    (bind _returnvalue (Game|Damage|ApplyDamage Other 0.35 0 0))
    (bind _asthird_person_character (Utilities|Casting|CastToThirdPersonCharacter (Game|GetPlayerCharacter 0)))
    (Default|ReceiveDamagePlayer _asthird_person_character _returnvalue)))

(fn ConstructionScript)